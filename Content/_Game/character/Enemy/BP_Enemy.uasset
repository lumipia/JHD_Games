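; BP_Enemy is a data-driven enemy character that configures itself from a data table on BeginPlay.
; It searches the table rows for one matching MonsterName, then applies that row's mesh, animation class, transform, montages and status.
; The row's HitBox value scales the base capsule radius and half height.
; Any damage plays the first montage at its stored play rate and makes the enemy jump.
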(event EventBeginPlay
  (bind _capsulecomponent (Variables|Collision|GetCapsuleComponent))
  (bind _mesh (Variables|Character|GetMesh))
  (bind _outrownames (DataTable|GetDataTableRowNames (Variables|Default|GetDataTale)))
  (bind _array_element (Utilities|Array|ForEachLoopwithBreak _outrownames :!label _label)
    (:LoopBody
      (bind _returnvalue (Utilities|GetDataTableRow (Variables|Default|GetDataTale) _array_element)
        (:then
          (if (Utilities|Name|Equal(Name) (.Name (Utilities|Struct|BreakF_Enemy _returnvalue)) (Variables|Default|GetMonsterName))
            (goto _label Break)))))
    (:Completed
      (bind _output_get (Variables|Default|SetEnemyInfo _returnvalue))
      (Variables|Default|SetMontages (.EnemyMontages (Utilities|Struct|BreakF_Enemy _output_get)))
      (Class|SkinnedMeshComponent|SetSkeletalMesh (Variables|Character|GetMesh) (.EnemyMesh (Utilities|Struct|BreakF_Enemy _output_get)) false)
      (Class|SkeletalMeshComponent|SetAnimClass _mesh (.EnemyAnimation (Utilities|Struct|BreakF_Enemy _output_get)))
      (Transformation|SetRelativeTransform _mesh (.Transform (Utilities|Struct|BreakF_Enemy _output_get)) false false)
      (Variables|Default|SetStatus (.Status (Utilities|Struct|BreakF_Enemy _output_get)))
      (Components|Capsule|SetCapsuleRadius _capsulecomponent (.Y (Math|Vector|BreakVector (* "88.000000,34.000000,0.000000" (.HitBox (Utilities|Struct|BreakF_Enemy _output_get))))) true)
      (Components|Capsule|SetCapsuleHalfHeight _capsulecomponent (.X (Math|Vector|BreakVector (* "88.000000,34.000000,0.000000" (.HitBox (Utilities|Struct|BreakF_Enemy _output_get))))) true))))

(event Game|Damage|EventAnyDamage
  (params (Damage :type Float%20%28single-precision%29) (DamageType :type Damage%20Type%20Object%20Reference) (InstigatedBy :type Controller%20Object%20Reference) (DamageCauser :type Actor%20Object%20Reference))
  (bind _montages (Variables|Default|GetMontages))
  (bind _output (Utilities|Array|Get(acopy) _montages))
  (Animation|PlayAnimMontage (.montage _output) (.playrate _output) "None")
  (Character|Jump))

(fn ConstructionScript)
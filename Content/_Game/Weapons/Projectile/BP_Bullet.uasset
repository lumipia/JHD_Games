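; BP_Bullet is a weapon projectile that damages characters it overlaps and has a three-second life span.
; Its Sphere overlap event ignores non-Character actors and the Attacker, then passes any other Character to the Attack function.
; Attack applies the Damage value to that character.
; The bullet is not destroyed on a hit in this graph, so it can damage several characters before expiring.
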(event OnComponentBeginOverlap(Sphere)
  (params (OverlappedComponent :type Primitive%20Component%20Object%20Reference) (OtherActor :type Actor%20Object%20Reference) (OtherComp :type Primitive%20Component%20Object%20Reference) (OtherBodyIndex :type Integer) (bFromSweep :type Boolean) (SweepResult :type Hit%20Result%20Structure%20%28by%20ref%29))
  (bind _ascharacter (Utilities|Casting|CastToCharacter OtherActor))
  (if (not (== _ascharacter (Variables|Default|GetAttacker)))
    (CallFunction|Attack _ascharacter)))

(event EventBeginPlay
  (|CallParentFunction)
  (Actor|SetLifeSpan 3.0))

(fn ConstructionScript
  (|CallParentFunction))

(fn Attack
  (params (DamagedActor :type Character%20Object%20Reference))
  (Game|Damage|ApplyDamage DamagedActor (Variables|Default|GetDamage) 0 0))
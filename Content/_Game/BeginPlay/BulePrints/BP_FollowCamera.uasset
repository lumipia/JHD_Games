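; BP_FollowCamera is a camera actor that follows the player character from a vertical offset with a fixed orientation.
; On BeginPlay it casts the first player character to BP_Player and caches it.
; Every Tick it sets its transform to the player's location plus Distance on Z, with constant rotation and unit scale, without smoothing or collision sweep.
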(event EventBeginPlay
  (bind _asbp_player (Utilities|Casting|CastToBP_Player (Game|GetPlayerCharacter 0)))
  (Variables|Default|SetPlayer _asbp_player))

(event EventTick
  (params (DeltaSeconds :type Float%20%28single-precision%29))
  (Transformation|SetActorTransform (Math|Transform|MakeTransform (+ (Math|Vector|MakeVector 0.0 0.0 (Variables|Default|GetDistance)) (Transformation|GetActorLocation (Variables|Default|GetPlayer))) "-90.000000,90.000000, 0")))

(fn ConstructionScript)